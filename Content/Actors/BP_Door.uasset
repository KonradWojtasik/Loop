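; BP_Door is a two-panel sliding door that opens and closes with sound, through OpenDoor and CloseDoor functions.
; On BeginPlay it async-loads both sounds and caches each panel's starting relative location.
; The functions set IsOpen, play or reverse the DoorAnimation timeline, and play the matching 2D sound.
; Timeline updates slide the panels apart along local X by offsetting them from the cached locations.
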(event `LoadAssets`
  (bind _object (`|LoadAsset` (`self.DoorOpenSound`))
    (:`then`
      (bind _object_2 (`|LoadAsset` (`self.DoorCloseSound`))
        (:`Completed`
          (set `self.DoorCloseSoundLoaded` (cast `SoundBase` _object_2 :!pure true)))))
    (:`Completed`
      (set `self.DoorOpenSoundLoaded` (cast `SoundBase` _object :!pure true)))))

(fn `CloseDoor`
  (set `self.IsOpen` false)
  (`TimelineComponent.Reverse` (`self.DoorAnimation`))
  (`GameplayStatics.PlaySound2D` (`self.DoorCloseSoundLoaded`) 1.0 1.0 0.0 null null))

(fn `OpenDoor`
  (set `self.IsOpen` true)
  (`TimelineComponent.Play` (`self.DoorAnimation`))
  (`GameplayStatics.PlaySound2D` (`self.DoorOpenSoundLoaded`) 1.0 1.0 0.0 null null))

(fn `ReceiveBeginPlay`
  (`self.LoadAssets`)
  (set `self.RelativeLocLeft` (`SceneComponent.RelativeLocation` (`self.DoorLeft`)))
  (set `self.RelativeLocRight` (`SceneComponent.RelativeLocation` (`self.DoorRight`))))

(fn `UserConstructionScript`)
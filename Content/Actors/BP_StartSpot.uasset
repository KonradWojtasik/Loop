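; BP_StartSpot is a pad that unlocks once all its linked pickups are hidden, then teleports the player to the next start spot.
; On BeginPlay it registers itself with each pickup, and ActivateButton lights the mesh and enables overlaps once none remain visible.
; Overlapping pauses player tick and moves them to NextStartSpot at PlayerStart height.
; Ending overlap resumes tick, resets the HUD timer and disables mesh overlaps.
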(fn `ActivateButton`
  (for _array_element (`self.Pickups`)
    (if (not (`Actor.bHidden` _array_element))
      (return)))
  (bind _returnvalue (`PrimitiveComponent.CreateDynamicMaterialInstance` (`self.StaticMesh`) 0 null "None"))
  (`MaterialInstanceDynamic.SetVectorParameterValue` _returnvalue "Color" (`self.ActivationColor`))
  (`MaterialInstanceDynamic.SetScalarParameterValue` _returnvalue "EmissiveMultiplier" 2.0)
  (set `PrimitiveComponent.bGenerateOverlapEvents` true (`self.StaticMesh`))
  (set `self.IsActive` true))

(fn `MeshBeginOverlap`
  (params (OverlappedComponent :type "PrimitiveComponent Object Reference") (OtherActor :type "Actor Object Reference") (OtherComp :type "PrimitiveComponent Object Reference") (OtherBodyIndex :type Integer) (bFromSweep :type Boolean) (SweepResult :type "HitResult Structure (by ref)"))
  (locals (TargetPlayer :type "/Game/Characters/BP_PlayerCharacter Object Reference"))
  (bind (_returnvalue_x _returnvalue_y) (`KismetMathLibrary.BreakVector` (`self.K2_GetActorLocation` (`self.NextStartSpot`))))
  (if (`self.IsActive`)
    (bind _asbp_player_character (cast `/Game/Characters/BP_PlayerCharacter` (`local.OtherActor`)))
    (set `local.TargetPlayer` _asbp_player_character)
    (`self.SetActorTickEnabled` (`local.TargetPlayer`) false)
    (`self.NextStartSpot`
      (:`then`
        (bind _returnvalue (`GameplayStatics.GetActorOfClass` "/Script/Engine.PlayerStart"))
        (bind (_returnvalue_x_2 _returnvalue_y_2 _returnvalue_z) (`KismetMathLibrary.BreakVector` (`self.K2_GetActorLocation` _returnvalue)))
        (`self.K2_SetActorLocationAndRotation` (`local.TargetPlayer`) (`KismetMathLibrary.MakeVector` _returnvalue_x _returnvalue_y _returnvalue_z) (`self.K2_GetActorRotation` (`self.NextStartSpot`)) false true))
      (:`else`))))

(fn `MeshEndOverlap`
  (params (OverlappedComponent :type "PrimitiveComponent Object Reference") (OtherActor :type "Actor Object Reference") (OtherComp :type "PrimitiveComponent Object Reference") (OtherBodyIndex :type Integer))
  (bind _asbp_player_character (cast `/Game/Characters/BP_PlayerCharacter` OtherActor))
  (if (not (`self.IsActorTickEnabled` _asbp_player_character))
    (`self.SetActorTickEnabled` _asbp_player_character true)
    (bind _asplayer_controller (cast `PlayerController` (`Pawn.GetController` _asbp_player_character)))
    (`/Game/UI/HUD_Custom.ResetTime` (cast `/Game/UI/HUD_Custom` (`PlayerController.GetHUD` _asplayer_controller) :!pure true) false)
    (set `PrimitiveComponent.bGenerateOverlapEvents` false (`self.StaticMesh`))))

(fn `ReceiveBeginPlay`
  (add `PrimitiveComponent.OnComponentBeginOverlap` (`self.StaticMesh`) (`|CreateDelegate` :!event `MeshBeginOverlap`))
  (add `PrimitiveComponent.OnComponentEndOverlap` (`self.StaticMesh`) (`|CreateDelegate` :!event `MeshEndOverlap`))
  (for _array_element (`self.Pickups`)
    (set `/Game/Actors/BP_Pickup.StartSpot` self _array_element)))

(fn `UserConstructionScript`)
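; BP_Pickup is a pickup actor that turns the player's recorded locations into an AI_PlayerCharacter when collected.
; It async-loads its Niagara effect on BeginPlay and plays it when BP_PlayerCharacter overlaps the mesh.
; The overlap appends a final point, spawns the AI at the path's start with that path, then clears the player's list.
; It then resets HUD time, hides itself, shows the GameState healing effect and calls the empty ApplyEffect hook.
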(event `LoadAssets`
  (bind _object (`|LoadAsset` (`self.PickupFX`))
    (:`Completed`
      (set `self.PickupFXLoaded` (cast `NiagaraSystem` _object :!pure true)))))

(fn `ApplyEffect`)

(fn `MeshBeginOverlap`
  (params (OverlappedComponent :type "PrimitiveComponent Object Reference") (OtherActor :type "Actor Object Reference") (OtherComp :type "PrimitiveComponent Object Reference") (OtherBodyIndex :type Integer) (bFromSweep :type Boolean) (SweepResult :type "HitResult Structure (by ref)"))
  (locals (TargetPlayer :type "/Game/Characters/BP_PlayerCharacter Object Reference"))
  (bind (_returnvalue_x _returnvalue_y) (`KismetMathLibrary.BreakVector` (`self.K2_GetActorLocation`)))
  (bind _locations (`/Game/Characters/BP_PlayerCharacter.Locations` (`local.TargetPlayer`)))
  (bind _locations_2 (`/Game/Characters/BP_PlayerCharacter.Locations` (`local.TargetPlayer`)))
  (bind (_output_x _output_y _output_z) (`KismetMathLibrary.BreakVector` (`|GetArrayItem` _locations (`KismetArrayLibrary.Array_LastIndex` _locations))))
  (bind _asbp_player_character (cast `/Game/Characters/BP_PlayerCharacter` OtherActor))
  (set `local.TargetPlayer` _asbp_player_character)
  (`NiagaraFunctionLibrary.SpawnSystemAtLocation` (`self.PickupFXLoaded`) (`self.K2_GetActorLocation`) (struct) (0.5 0.5 0.5))
  (`KismetArrayLibrary.Array_Add` (`/Game/Characters/BP_PlayerCharacter.Locations` (`local.TargetPlayer`)) (`KismetMathLibrary.MakeVector` _returnvalue_x _returnvalue_y _output_z))
  (`|SpawnActorFromClass` "/Game/Characters/AI/AI_PlayerCharacter.AI_PlayerCharacter_C" (`KismetMathLibrary.Conv_VectorToTransform` (`|GetArrayItem` _locations_2)) "Undefined" "MultiplyWithRoot" null _locations_2 null)
  (`KismetArrayLibrary.Array_Clear` (`/Game/Characters/BP_PlayerCharacter.Locations` (`local.TargetPlayer`)))
  (`/Game/UI/HUD_Custom.ResetTime` (cast `/Game/UI/HUD_Custom` (`PlayerController.GetHUD` (cast `PlayerController` (`Pawn.GetController` (`local.TargetPlayer`)) :!pure true)) :!pure true) false)
  (`self.SetActorHiddenInGame` true)
  (set `PrimitiveComponent.bGenerateOverlapEvents` false (`self.StaticMesh`))
  (`/Game/Core/BP_GameState_Custom.ShowHealingEffect` (cast `/Game/Core/BP_GameState_Custom` (`GameplayStatics.GetGameState`) :!pure true))
  (`self.ApplyEffect`))

(fn `ReceiveBeginPlay`
  (`self.LoadAssets`)
  (add `PrimitiveComponent.OnComponentBeginOverlap` (`self.StaticMesh`) (`|CreateDelegate` :!event `MeshBeginOverlap`)))

(fn `UserConstructionScript`)
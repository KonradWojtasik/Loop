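; BP_Button is a pressure-plate style button that opens its linked doors while something overlaps its mesh.
; Begin overlap opens every closed door in its Doors array and plays a 2D click sound unless muted; end overlap closes every open one.
; The sound is async-loaded from a soft reference at BeginPlay, where the overlap events are also bound.
; Any overlapping actor triggers it, and occupants are not counted.
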(event `LoadAssets`
  (bind _object (`|LoadAsset` (`self.ButtonSound`))
    (:`Completed`
      (set `self.ButtonSoundLoaded` (cast `SoundBase` _object :!pure true)))))

(fn ` ButtonEndOverlap`
  (params (OverlappedComponent :type "PrimitiveComponent Object Reference") (OtherActor :type "Actor Object Reference") (OtherComp :type "PrimitiveComponent Object Reference") (OtherBodyIndex :type Integer))
  (locals (TargetPlayer :type "/Game/Characters/BP_PlayerCharacter Object Reference"))
  (for _array_element (`self.Doors`)
    (if (`/Game/Actors/BP_Door.IsOpen` _array_element)
      (`/Game/Actors/BP_Door.CloseDoor` _array_element))))

(fn `ButtonBeginOverlap`
  (params (OverlappedComponent :type "PrimitiveComponent Object Reference") (OtherActor :type "Actor Object Reference") (OtherComp :type "PrimitiveComponent Object Reference") (OtherBodyIndex :type Integer) (bFromSweep :type Boolean) (SweepResult :type "HitResult Structure (by ref)"))
  (locals (TargetPlayer :type "/Game/Characters/BP_PlayerCharacter Object Reference"))
  (for _array_element (`self.Doors`)
    (if (not (`/Game/Actors/BP_Door.IsOpen` _array_element))
      (`/Game/Actors/BP_Door.OpenDoor` _array_element)))
  (if (not (`self.isMuted`))
    (`GameplayStatics.PlaySound2D` (`self.ButtonSoundLoaded`) 1.0 1.0 0.0 null null)))

(fn `ReceiveBeginPlay`
  (`self.LoadAssets`)
  (add `PrimitiveComponent.OnComponentBeginOverlap` (`self.StaticMesh`) (`|CreateDelegate` :!event `ButtonBeginOverlap`))
  (add `PrimitiveComponent.OnComponentEndOverlap` (`self.StaticMesh`) (`|CreateDelegate` :!event ` ButtonEndOverlap`)))

(fn `UserConstructionScript`)
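; Custom GameState that loads the save and music at begin play and handles the game-over respawn.
; Glitch and healing effects toggle weighted post-process materials on the level's PostProcessVolume, with one-second timers.
; GameOver teleports the player to the saved BP_StartSpot, restoring its pickups and resetting other spots by ID, or to PlayerStart with all pickups restored.
; It also destroys AI_PlayerCharacter actors and resets the HUD time.
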(event `LoadAssets`
  (bind _object (`|LoadAsset` (`self.Music`))
    (:`Completed`
      (`GameplayStatics.SpawnSound2D` (cast `SoundBase` _object :!pure true) 1.0 1.0 0.0 null))))

(fn `GameOver`
  (locals (TargetPlayer :type "/Game/Characters/BP_PlayerCharacter Object Reference") (TargetSpot :type "/Game/Actors/BP_StartSpot Object Reference") (TargetStart :type "PlayerStart Object Reference"))
  (bind (_returnvalue_location _returnvalue_rotation) (`KismetMathLibrary.BreakTransform` (`self.GetTransform` (`local.TargetStart`))))
  (bind (_returnvalue_x _returnvalue_y _returnvalue_z) (`KismetMathLibrary.BreakVector` (`self.K2_GetActorLocation` (`local.TargetStart`))))
  (bind (_returnvalue_x_2 _returnvalue_y_2) (`KismetMathLibrary.BreakVector` (`self.K2_GetActorLocation` (`local.TargetSpot`))))
  (set `local.TargetPlayer` (cast `/Game/Characters/BP_PlayerCharacter` (`PlayerState.GetPawn` (`|GetArrayItem` (`self.PlayerArray`))) :!pure true))
  (`self.SetActorTickEnabled` (`local.TargetPlayer`) false)
  (`KismetArrayLibrary.Array_Clear` (`/Game/Characters/BP_PlayerCharacter.Locations` (`local.TargetPlayer`)))
  (`KismetSystemLibrary.K2_ClearAndInvalidateTimerHandle` (`self.HealingTimer`))
  (`self.HideHealingEffect`)
  (`self.ShowGlitchEffect`)
  (`|ExecutionSequence`
    (:`then_0`
      (bind _result (`/Game/Core/GameInstance_Custom.GetSaveGame` (cast `/Game/Core/GameInstance_Custom` (`GameplayStatics.GetGameInstance`) :!pure true)))
      (`/Engine/EditorBlueprintResources/StandardMacros.IsValid` _result
        (:`Is Valid`
          (bind _outactors (`GameplayStatics.GetAllActorsOfClass` "/Game/Actors/BP_StartSpot.BP_StartSpot_C"))
          (for _array_element _outactors
            (if (== (`/Game/Actors/BP_StartSpot.ID` _array_element) (`/Game/Core/Misc/SaveGame_Custom.StartSpotID` _result))
              (set `local.TargetSpot` _array_element)
              (break)))
          (bind _returnvalue (`GameplayStatics.GetActorOfClass` "/Script/Engine.PlayerStart"))
          (set `local.TargetStart` _returnvalue)
          (bind _targetspot (`local.TargetSpot`)
            (:`then`
              (set `/Game/Actors/BP_StartSpot.IsActive` false _targetspot)
              (`/Game/Actors/BP_StartSpot.SetActiveDirectly` _targetspot true false)
              (`self.K2_SetActorLocationAndRotation` (`local.TargetPlayer`) (`KismetMathLibrary.MakeVector` _returnvalue_x_2 _returnvalue_y_2 _returnvalue_z) (`self.K2_GetActorRotation` (`local.TargetSpot`)) false true)
              (set `PrimitiveComponent.bGenerateOverlapEvents` true (`/Game/Actors/BP_StartSpot.StaticMesh` (`local.TargetSpot`)))
              (for _array_element_2 (`/Game/Actors/BP_StartSpot.Pickups` (`local.TargetSpot`))
                (`self.SetActorHiddenInGame` _array_element_2 false)
                (set `PrimitiveComponent.bGenerateOverlapEvents` true (`/Game/Actors/BP_Pickup.StaticMesh` _array_element_2)))
              (bind _outactors_2 (`GameplayStatics.GetAllActorsOfClass` "/Game/Actors/BP_StartSpot.BP_StartSpot_C"))
              (for _array_element_3 _outactors_2
                (if (!= (`local.TargetSpot`) _array_element_3)
                  (if (< (`/Game/Actors/BP_StartSpot.ID` _array_element_3) (`/Game/Actors/BP_StartSpot.ID` (`local.TargetSpot`)))
                    (`/Game/Actors/BP_StartSpot.SetActiveDirectly` _array_element_3 true true)
                    (else
                      (`/Game/Actors/BP_StartSpot.SetActiveDirectly` _array_element_3 false false)
                      (for _array_element_4 (`/Game/Actors/BP_StartSpot.Doors` _array_element_3)
                        (set `/Game/Actors/BP_Door.isMuted` false _array_element_4))
                      (for _array_element_5 (`/Game/Actors/BP_StartSpot.Buttons` _array_element_3)
                        (set `/Game/Actors/BP_Button.isMuted` false _array_element_5)))))))
            (:`else`
              (`self.K2_SetActorLocationAndRotation` (`local.TargetPlayer`) _returnvalue_location _returnvalue_rotation false true)
              (bind _outactors_3 (`GameplayStatics.GetAllActorsOfClass` "/Game/Actors/BP_Pickup.BP_Pickup_C"))
              (for _array_element_6 _outactors_3
                (`self.SetActorHiddenInGame` _array_element_6 false)
                (set `PrimitiveComponent.bGenerateOverlapEvents` true (`/Game/Actors/BP_Pickup.StaticMesh` _array_element_6))))))))
    (:`then_1`
      (bind _outactors_4 (`GameplayStatics.GetAllActorsOfClass` "/Game/Characters/AI/AI_PlayerCharacter.AI_PlayerCharacter_C"))
      (for _array_element_7 _outactors_4
        (`self.K2_DestroyActor` _array_element_7))
      (`/Game/UI/HUD_Custom.ResetTime` (cast `/Game/UI/HUD_Custom` (`PlayerController.GetHUD` (cast `PlayerController` (`Pawn.GetController` (`local.TargetPlayer`)) :!pure true)) :!pure true) true))))

(fn `HideGlitchEffect`
  (bind _returnvalue (`GameplayStatics.GetActorOfClass` "/Script/Engine.PostProcessVolume"))
  (setmembers `WeightedBlendable` :`StructRef` (`|GetArrayItem` (`.Array` (break `WeightedBlendables` (`.WeightedBlendables` (break `PostProcessSettings` (`PostProcessVolume.Settings` _returnvalue)))))) :`Weight` 0.0))

(fn `HideHealingEffect`
  (bind _returnvalue (`GameplayStatics.GetActorOfClass` "/Script/Engine.PostProcessVolume"))
  (setmembers `WeightedBlendable` :`StructRef` (`|GetArrayItem` (`.Array` (break `WeightedBlendables` (`.WeightedBlendables` (break `PostProcessSettings` (`PostProcessVolume.Settings` _returnvalue))))) 1) :`Weight` 0.0))

(fn `ReceiveBeginPlay`
  (`/Game/Core/GameInstance_Custom.LoadSaveGame` (cast `/Game/Core/GameInstance_Custom` (`GameplayStatics.GetGameInstance`) :!pure true))
  (`self.ShowGlitchEffect`)
  (`self.LoadAssets`))

(fn `ShowGlitchEffect`
  (bind _returnvalue (`GameplayStatics.GetActorOfClass` "/Script/Engine.PostProcessVolume"))
  (setmembers `WeightedBlendable` :`StructRef` (`|GetArrayItem` (`.Array` (break `WeightedBlendables` (`.WeightedBlendables` (break `PostProcessSettings` (`PostProcessVolume.Settings` _returnvalue)))))) :`Weight` 1.0)
  (bind _returnvalue_2 (`KismetSystemLibrary.K2_SetTimerDelegate` (`|CreateDelegate` :!event `HideGlitchEffect`) 1.0))
  (set `self.GlitchTimer` _returnvalue_2))

(fn `ShowHealingEffect`
  (bind _returnvalue (`GameplayStatics.GetActorOfClass` "/Script/Engine.PostProcessVolume"))
  (setmembers `WeightedBlendable` :`StructRef` (`|GetArrayItem` (`.Array` (break `WeightedBlendables` (`.WeightedBlendables` (break `PostProcessSettings` (`PostProcessVolume.Settings` _returnvalue))))) 1) :`Weight` 1.0)
  (bind _returnvalue_2 (`KismetSystemLibrary.K2_SetTimerDelegate` (`|CreateDelegate` :!event `HideHealingEffect`) 1.0))
  (set `self.HealingTimer` _returnvalue_2))

(fn `UserConstructionScript`)
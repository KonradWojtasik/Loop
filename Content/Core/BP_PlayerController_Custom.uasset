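; Custom player controller that handles pause and quick-restart input and fixes the view to a camera actor.
; On local BeginPlay it sets game-only input, adds the default Enhanced Input mapping context and switches the view target to the CameraActor it finds.
; Pause toggles the menu through the custom HUD, while quick restart calls GameOver on the custom game state.
; A debug T key, disabled in distribution builds, toggles whether the controlled pawn can be damaged.
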(event `EnhancedInput|/Game/Core/Input/Actions/IA_Menu_Pause`
  (params (ActionValue :type Boolean) (ElapsedSeconds :type "Float (double-precision)") (TriggeredSeconds :type "Float (double-precision)") (InputAction :type "InputAction Object Reference" :default "/Game/Core/Input/Actions/IA_Menu_Pause.IA_Menu_Pause"))
  (:`Started`
    (bind _ashud_custom (cast `/Game/UI/HUD_Custom` (`self.GetHUD`)))
    (`/Game/UI/HUD_Custom.TogglePauseMenu` _ashud_custom)))

(event `EnhancedInput|/Game/Core/Input/Actions/IA_QuickRestart`
  (params (ActionValue :type Boolean) (ElapsedSeconds :type "Float (double-precision)") (TriggeredSeconds :type "Float (double-precision)") (InputAction :type "InputAction Object Reference" :default "/Game/Core/Input/Actions/IA_QuickRestart.IA_QuickRestart"))
  (:`Started`
    (bind _asbp_game_state_custom (cast `/Game/Core/BP_GameState_Custom` (`GameplayStatics.GetGameState`)))
    (`/Game/Core/BP_GameState_Custom.GameOver` _asbp_game_state_custom)))

(event `Key|T` :consume false :overrideparent false
  (params (Key :type "Key Structure"))
  (bind _returnvalue (`self.K2_GetPawn`))
  ;[1 0 0 0] Debug
  (:`Pressed`
    (if (not (`KismetSystemLibrary.IsPackagedForDistribution`))
      (bind _output_get (set `Actor.bCanBeDamaged` (not (`Actor.bCanBeDamaged` _returnvalue)) _returnvalue))
      (`KismetSystemLibrary.PrintString` (`KismetStringLibrary.Conv_BoolToString` _output_get) true false (struct :`R` 1.0 :`G` 1.0 :`A` 1.0) 5.0 "Damage"))))

(fn `ReceiveBeginPlay`
  (if (`self.IsLocalController`)
    (`WidgetBlueprintLibrary.SetInputMode_GameOnly` self)
    (`EnhancedInputSubsystemInterface.AddMappingContext` (pcsubsystem `EnhancedInputLocalPlayerSubsystem` self) "/Game/Core/Input/IMC_Default.IMC_Default" 0 (struct))
    (bind _returnvalue (`GameplayStatics.GetActorOfClass` "/Script/Engine.CameraActor"))
    (`self.SetViewTargetWithBlend` _returnvalue)))

(fn `UserConstructionScript`)
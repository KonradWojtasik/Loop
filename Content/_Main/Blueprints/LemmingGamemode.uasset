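; Game mode for a round-based lemming puzzle where the player works alongside replays of their earlier runs.
; BeginPlay orders spawn points, loads the saved round and spawns one lemming per round, possessing the newest.
; While the gate is open, Tick records the player's state and replays past lemmings frame by frame, marking desyncs when interact availability differs.
; EndRound saves the recording and reloads the level; completing the final round clears the save.
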(event `StartRound`
  (bind _roundnum (`self.LoadGame`))
  (bind _output_get (set `self.LemmingNum` _roundnum))
  (`self.SpawnLemming` _output_get)
  (`self.OpenGate`))

(event `ResetRound`
  (`GameplayStatics.SaveGameToSlot` (`self.LemmingSaveGame`) "Lemming")
  (bind _returnvalue (`GameplayStatics.GetCurrentLevelName` true))
  (`GameplayStatics.OpenLevel` (`KismetStringLibrary.Conv_StringToName` _returnvalue))
  (`KismetSystemLibrary.PrintString` "Reset Current Level"))

(event `EndRound`
  (`self.SaveGame`)
  (bind _returnvalue (`GameplayStatics.GetCurrentLevelName` true))
  (`GameplayStatics.OpenLevel` (`KismetStringLibrary.Conv_StringToName` _returnvalue)))

(event `self.ReceiveBeginPlay`
  (`self.OrderSpawnPoints`)
  (`self.StartRound`))

(event `self.ReceiveTick`
  (params (DeltaSeconds :type "Float (single-precision)"))
  (`/Engine/EditorBlueprintResources/StandardMacros.Gate` true :!label _label
    (:`Exit`
      (`self.RecordLemming` false)
      (`self.ReplayLemmingManager`))))

(event `OpenGate`
  (goto _label :!via `Open`))

(fn `ClearSavedGames`
  ;[1 0 0] BE VERY CAREFUL WITH THIS!!! If this is called (in the Level BP's), it will not work in a packaged build
  (bind _returnvalue (`GameplayStatics.DoesSaveGameExist` "Lemming"))
  (`KismetSystemLibrary.PrintString` (`KismetStringLibrary.Conv_BoolToString` _returnvalue) true true (struct :`R` 1.0 :`G` 0.047563 :`A` 1.0) 200.0)
  (`GameplayStatics.DeleteGameInSlot` "Lemming")
  (`KismetSystemLibrary.PrintString` "DELETING SAVE FILES" true true (struct :`R` 1.0 :`G` 0.905019 :`A` 1.0) 200.0))

(fn `LoadGame`
  (returns (RoundNum :type Integer))
  (bind _returnvalue (`GameplayStatics.DoesSaveGameExist` "Lemming"))
  (if (not _returnvalue)
    (`self.SaveGame`))
  (bind _returnvalue_2 (`GameplayStatics.LoadGameFromSlot` "Lemming"))
  (bind _aslemming_save_game (cast `/Game/_Main/Blueprints/LemmingSaveGame` _returnvalue_2))
  (set `self.LemmingSaveGame` _aslemming_save_game)
  (bind _roundnum (`/Game/_Main/Blueprints/LemmingSaveGame.RoundNum` _aslemming_save_game))
  (bind _returnvalue_3 (+ _roundnum 1))
  (if (>= (`self.MaxLemmings`) _returnvalue_3)
    (set `self.RoundNum` _returnvalue_3)
    (set `self.LemmingInfoReplay1` (`/Game/_Main/Blueprints/LemmingSaveGame.LemmingInfoReplay1` _aslemming_save_game))
    (set `self.LemmingInfoReplay2` (`/Game/_Main/Blueprints/LemmingSaveGame.LemmingInfoReplay2` _aslemming_save_game))
    (set `self.LemmingInfoReplay3` (`/Game/_Main/Blueprints/LemmingSaveGame.LemmingInfoReplay3` _aslemming_save_game))
    (set `self.LemmingInfoReplay4` (`/Game/_Main/Blueprints/LemmingSaveGame.LemmingInfoReplay4` _aslemming_save_game))
    (return (`self.RoundNum`))
    (else
      (`self.ResetRound`)
      (return _roundnum))))

(fn `OrderSpawnPoints`
  (bind _outactors (`GameplayStatics.GetAllActorsOfClass` "/Game/_Main/Blueprints/Actors/BP_LemmingSpawnPoint.BP_LemmingSpawnPoint_C"))
  (set `self.MaxLemmings` (`KismetArrayLibrary.Array_Length` _outactors))
  (for _array_element _outactors
    (`KismetArrayLibrary.Array_Set` (`self.PlayerStarts`) (`/Game/_Main/Blueprints/Actors/BP_LemmingSpawnPoint.SpawnNum` _array_element) _array_element)))

(fn `RecordLemming`
  (params (`Interact?` :type Boolean))
  (bind _playerpawn (`self.PlayerPawn`))
  (`/Engine/EditorBlueprintResources/StandardMacros.IsValid` _playerpawn
    (:`Is Valid`
      (`KismetArrayLibrary.Array_Add` (`self.LemmingInfoRecord`) (make `/Game/_Main/Blueprints/LemmingDataStruct` (`SceneComponent.K2_GetComponentToWorld` (`Actor.RootComponent` _playerpawn)) (`MovementComponent.Velocity` (`Pawn.GetMovementComponent` _playerpawn)) (`/Game/_Main/Character/Lemming.IsFalling?` _playerpawn) (`/Game/_Main/Character/Lemming.CanInteract?` _playerpawn) `Interact?` (`SceneComponent.K2_GetComponentRotation` (`/Game/_Main/Character/Lemming.Camera` _playerpawn)))))))

(fn `ReplayLemming`
  (params (InfoReplay :type "Array of /Game/_Main/Blueprints/LemmingDataStruct Structure") (Lemming :type "/Game/_Main/Character/Lemming Object Reference"))
  (bind _lemming (`local.Lemming`))
  (bind _lemming_2 (`local.Lemming`))
  (bind (_output_transform _output_velocity _output_isfalling_ _output_caninteract_ _output_interact_ _output_camera) (break `/Game/_Main/Blueprints/LemmingDataStruct` (`|GetArrayItem` (`local.InfoReplay`) (`self.Index`))))
  (`/Engine/EditorBlueprintResources/StandardMacros.IsValid` Lemming
    (:`Is Valid`
      (if (and (>= (`self.RoundNum`) 2) (not (`/Game/_Main/Character/Lemming.Desynced?` Lemming)) (> (`KismetArrayLibrary.Array_Length` InfoReplay) (`self.Index`)))
        ;[1 1 1] Get and compare to what is happening
        (`|ExecutionSequence`
          (:`then_0`
            ;[1 1 1] Set and then compare and make sure tp is good
            (bind _sweephitresult (`SceneComponent.K2_SetWorldTransform` (`Actor.RootComponent` _lemming_2) _output_transform true false))
            (`SceneComponent.K2_SetWorldRotation` (`/Game/_Main/Character/Lemming.Camera` _lemming_2) _output_camera false false)
            (set `MovementComponent.Velocity` _output_velocity (`Pawn.GetMovementComponent` _lemming_2)))
          (:`then_1`
            (if (!= _output_caninteract_ (`/Game/_Main/Character/Lemming.CanInteract?` _lemming))
              (`/Game/_Main/Character/Lemming.SetDesynced` _lemming)
              (`KismetSystemLibrary.PrintString` "desynced - can interact" true true (struct :`G` 0.377854 :`B` 1.0 :`A` 1.0) 10.0)))
          (:`then_2`
            (if _output_interact_
              (`/Game/_Main/Character/Lemming.Interact` _lemming)
              (`KismetSystemLibrary.PrintString` "interacted" true true (struct :`R` 0.514425 :`G` 1.0 :`B` 0.289067 :`A` 1.0) 5.0))))))))

(fn `ReplayLemmingManager`
  (set `self.Index` (+ (`self.Index`) 1))
  (`|ExecutionSequence`
    (:`then_0`
      (`self.ReplayLemming` (`self.LemmingInfoReplay1`) (`self.Lemming1`)))
    (:`then_1`
      (`self.ReplayLemming` (`self.LemmingInfoReplay2`) (`self.Lemming2`)))
    (:`then_2`
      (`self.ReplayLemming` (`self.LemmingInfoReplay3`) (`self.Lemming3`)))
    (:`then_3`
      (`self.ReplayLemming` (`self.LemmingInfoReplay4`) (`self.Lemming4`)))))

(fn `SaveGame`
  (bind _lemmingsavegame (`self.LemmingSaveGame`))
  (bind _lemminginforecord (`self.LemmingInfoRecord`))
  (bind _lemmingsavegame_2 (`self.LemmingSaveGame`))
  (`/Engine/EditorBlueprintResources/StandardMacros.IsValid` _lemmingsavegame_2
    (:`Is Valid`
      _)
    (:`Is Not Valid`
      (bind _returnvalue (`GameplayStatics.CreateSaveGameObject` "/Game/_Main/Blueprints/LemmingSaveGame.LemmingSaveGame_C"))
      (set `self.LemmingSaveGame` _returnvalue)))
  (bind _output_get (set `/Game/_Main/Blueprints/LemmingSaveGame.RoundNum` (`self.RoundNum`) _lemmingsavegame_2))
  (if (>= (`self.MaxLemmings`) (+ _output_get 1))
    (switch `int` _output_get
      (:`Default`
        (bind _returnvalue_2 (`GameplayStatics.SaveGameToSlot` (`self.LemmingSaveGame`) "Lemming" :!label _label))
        (if _returnvalue_2
          (`KismetSystemLibrary.PrintString` (`KismetStringLibrary.Concat_StrStr` "Round " (`KismetStringLibrary.Conv_IntToString` (`self.RoundNum`)) " saved") true true (struct :`G` 1.0 :`B` 0.016063 :`A` 1.0) 20.0)
          (else
            (`KismetSystemLibrary.PrintString` (`KismetStringLibrary.Concat_StrStr` "Round " (`KismetStringLibrary.Conv_IntToString` (`self.RoundNum`)) " not saved") true true (struct :`R` 1.0 :`B` 0.002776 :`A` 1.0) 20.0))))
      (:`1`
        (set `/Game/_Main/Blueprints/LemmingSaveGame.LemmingInfoReplay1` _lemminginforecord _lemmingsavegame)
        (goto _label))
      (:`2`
        (set `/Game/_Main/Blueprints/LemmingSaveGame.LemmingInfoReplay2` _lemminginforecord _lemmingsavegame)
        (goto _label))
      (:`3`
        (set `/Game/_Main/Blueprints/LemmingSaveGame.LemmingInfoReplay3` _lemminginforecord _lemmingsavegame)
        (goto _label))
      (:`4`
        (set `/Game/_Main/Blueprints/LemmingSaveGame.LemmingInfoReplay4` _lemminginforecord _lemmingsavegame)
        (goto _label))
      (:`5`
        (`self.ClearSavedGames`)
        (`KismetSystemLibrary.PrintString` "GAME COMPLETED" true true (struct :`R` 0.025236 :`G` 1.0 :`A` 1.0) 5.0)))
    (else
      (`self.ClearSavedGames`))))

(fn `SpawnLemming`
  (params (Round :type Integer))
  (locals (LemmingCount :type Integer :default 1))
  (bind _masterlemming (`self.MasterLemming`))
  (bind _returnvalue (`self.GetTransform` (`|GetArrayItem` (`self.PlayerStarts`) (`local.LemmingCount`))))
  ;[1 1 1] Spawns the correct number of lemmings per round
  (if (>= Round (`local.LemmingCount`)) :!label _label
    (switch `int` (`local.LemmingCount`)
      (:`1`
        (bind _returnvalue_2 (`|SpawnActorFromClass` "/Game/_Main/Character/Lemming.Lemming_C" _returnvalue "AlwaysSpawn" "MultiplyWithRoot" null (`local.LemmingCount`) null))
        (bind _output_get (set `self.Lemming1` _returnvalue_2))
        (`Controller.Possess` (cast `/Game/Core/BP_PlayerController_Custom` (`GameplayStatics.GetPlayerController` 0) :!pure true) _output_get)
        (set `self.PlayerPawn` _output_get)
        (`/Engine/EditorBlueprintResources/StandardMacros.IncrementInt` (`local.LemmingCount`)
          (:`  `
            (goto _label))))
      (:`2`
        (bind _returnvalue_3 (`|SpawnActorFromClass` "/Game/_Main/Character/Lemming.Lemming_C" _returnvalue "AlwaysSpawn" "MultiplyWithRoot" null (`local.LemmingCount`) null))
        (bind _output_get_2 (set `self.Lemming2` _returnvalue_3))
        (`Controller.Possess` (cast `/Game/Core/BP_PlayerController_Custom` (`GameplayStatics.GetPlayerController` 0) :!pure true) _output_get_2)
        (set `self.PlayerPawn` _output_get_2)
        (`/Engine/EditorBlueprintResources/StandardMacros.IncrementInt` (`local.LemmingCount`)
          (:`  `
            (goto _label))))
      (:`3`
        (bind _returnvalue_4 (`|SpawnActorFromClass` "/Game/_Main/Character/Lemming.Lemming_C" _returnvalue "AlwaysSpawn" "MultiplyWithRoot" null (`local.LemmingCount`) null))
        (bind _output_get_3 (set `self.Lemming3` _returnvalue_4))
        (`Controller.Possess` (cast `/Game/Core/BP_PlayerController_Custom` (`GameplayStatics.GetPlayerController` 0) :!pure true) _output_get_3)
        (set `self.PlayerPawn` _output_get_3)
        (`/Engine/EditorBlueprintResources/StandardMacros.IncrementInt` (`local.LemmingCount`)
          (:`  `
            (goto _label))))
      (:`4`
        (bind _returnvalue_5 (`|SpawnActorFromClass` "/Game/_Main/Character/Lemming.Lemming_C" _returnvalue "AlwaysSpawn" "MultiplyWithRoot" null (`local.LemmingCount`) null))
        (bind _output_get_4 (set `self.Lemming4` _returnvalue_5))
        (`Controller.Possess` (cast `/Game/Core/BP_PlayerController_Custom` (`GameplayStatics.GetPlayerController` 0) :!pure true) _output_get_4)
        (set `self.PlayerPawn` _output_get_4)
        (`/Engine/EditorBlueprintResources/StandardMacros.IncrementInt` (`local.LemmingCount`)
          (:`  `
            (goto _label))))
      (:`5`
        ;;[1 0 0] Master Lemming is deprecated in BeginPlay
        (`Controller.Possess` (cast `/Game/Core/BP_PlayerController_Custom` (`GameplayStatics.GetPlayerController` 0) :!pure true) _masterlemming)
        (set `self.PlayerPawn` _masterlemming)))))

(fn `UserConstructionScript`)
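; LemmingController is the input controller for the Lemming game, turning hard-wired key presses into round and character actions.
; P, R and X call the LemmingGamemode to end the round, reset it or clear saved games.
; E triggers Interaction on player 0's Lemming character.
; It holds no logic of its own, as each key casts to its target and forwards the call.
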(event `Key|P`
  (params (Key :type "Key Structure"))
  (:`Pressed`
    (bind _aslemming_gamemode (cast `/Game/_Main/Blueprints/LemmingGamemode` (`GameplayStatics.GetGameMode`)))
    (`/Game/_Main/Blueprints/LemmingGamemode.EndRound` _aslemming_gamemode)))

(event `self.ReceiveBeginPlay`)

(event `Key|R`
  (params (Key :type "Key Structure"))
  (:`Pressed`
    (bind _aslemming_gamemode (cast `/Game/_Main/Blueprints/LemmingGamemode` (`GameplayStatics.GetGameMode`)))
    (`/Game/_Main/Blueprints/LemmingGamemode.ResetRound` _aslemming_gamemode)))

(event `Key|X`
  (params (Key :type "Key Structure"))
  (:`Pressed`
    (bind _aslemming_gamemode (cast `/Game/_Main/Blueprints/LemmingGamemode` (`GameplayStatics.GetGameMode`)))
    (`/Game/_Main/Blueprints/LemmingGamemode.ClearSavedGames` _aslemming_gamemode)))

(event `Key|E`
  (params (Key :type "Key Structure"))
  (:`Pressed`
    (bind _aslemming (cast `/Game/_Main/Character/Lemming` (`GameplayStatics.GetPlayerCharacter` 0)))
    (`/Game/_Main/Character/Lemming.Interaction` _aslemming)))

(fn `UserConstructionScript`)